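; Player controller that sets up Enhanced Input for the player character and forwards move input to it.
; On BeginPlay it adds the IMC_Main mapping context and caches player 0's character as BP_Player.
; The IA_Move action passes its X and Z axis values to the player's Movement function as left-right and vertical input.
; Some leftover axis comparison nodes are disconnected.
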(event Input|EnhancedActionEvents|EnhancedInputActionIA_Move
  (params (ActionValue :type Vector :default "0, 0, 0") (ElapsedSeconds :type Float%20%28double-precision%29) (TriggeredSeconds :type Float%20%28double-precision%29) (InputAction :type Input%20Action%20Object%20Reference :default "/Game/Character/Inputs/Main/IA_Move.IA_Move"))
  (bind (_x _y _z) (Math|Vector|BreakVector ActionValue))
  (Default|Movement (Variables|Default|GetAs%20BP%20Player) _z _x 0.0))

(event Input|EnhancedActionEvents|EnhancedInputActionIA_Move
  (params (ActionValue :type Vector :default "0, 0, 0") (ElapsedSeconds :type Float%20%28double-precision%29) (TriggeredSeconds :type Float%20%28double-precision%29) (InputAction :type Input%20Action%20Object%20Reference :default "/Game/Character/Inputs/Main/IA_Move.IA_Move")))

(event EventBeginPlay
  (Input|AddMappingContext (PlayerController|LocalPlayerSubsystems|GetEnhancedInputLocalPlayerSubsystem) "/Game/Character/Inputs/IMC_Main.IMC_Main" 0 "(bIgnoreAllPressedKeysUntilRelease=True,bForceImmediately=False,bNotifyUserSettings=False)")
  (bind _asbp_player (Utilities|Casting|CastToBP_Player (Game|GetPlayerCharacter 0)))
  (Variables|Default|SetAs%20BP%20Player _asbp_player))

(fn ConstructionScript)