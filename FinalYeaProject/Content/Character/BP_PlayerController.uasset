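; BP_PlayerController is a player controller Blueprint that sets up Enhanced Input and prints move input for debugging.
; On BeginPlay it adds the IMC_Main mapping context to the local player's Enhanced Input subsystem.
; While IA_Move triggers, it prints each axis of the action value with a label; it applies no movement, and the construction script is empty.
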(event Input|EnhancedActionEvents|EnhancedInputActionIA_Move
  (params (ActionValue :type Vector :default "0, 0, 0") (ElapsedSeconds :type Float%20%28double-precision%29) (TriggeredSeconds :type Float%20%28double-precision%29) (InputAction :type Input%20Action%20Object%20Reference :default "/Game/Character/Inputs/Main/IA_Move.IA_Move"))
  (bind (_x _y _z) (Math|Vector|BreakVector ActionValue))
  (:Triggered
    (Development|PrintString (Utilities|String|Append "X:" (Utilities|String|ToString(Float) _x)))
    (Development|PrintString (Utilities|String|Append "Y:" (Utilities|String|ToString(Float) _y)))
    (Development|PrintString (Utilities|String|Append "Z:" (Utilities|String|ToString(Float) _z)))))

(event EventBeginPlay
  (Input|AddMappingContext (PlayerController|LocalPlayerSubsystems|GetEnhancedInputLocalPlayerSubsystem) "/Game/Character/Inputs/IMC_Main.IMC_Main" 0 "(bIgnoreAllPressedKeysUntilRelease=True,bForceImmediately=False,bNotifyUserSettings=False)"))

(fn ConstructionScript)